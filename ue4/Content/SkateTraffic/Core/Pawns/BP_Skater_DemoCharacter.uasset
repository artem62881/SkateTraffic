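; Demo skater pawn for SkateTraffic that adds speed-driven camera effects and skateboard audio.
; Each tick it sets camera FOV and post-process blur, easing both from default toward maximum as velocity climbs past a threshold.
; When grounded, it spawns land and ride sounds once at the capsule's base, stopping the ride sound while falling or when destroyed.
; Ride pitch is recalculated from speed but applied only when the sound spawns.
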(event `self.ReceiveBeginPlay`
  (set `self.DefaultFOV` (`CameraComponent.FieldOfView` (`self.CameraComponent`))))

(event `self.ReceiveTick`
  (params (DeltaSeconds :type "Float (single-precision)"))
  (bind _ridesoundref (`self.RideSoundRef`))
  (`self.Set Player Camera BlurAndFOV`)
  (if (not (`NavMovementComponent.IsFalling` (`self.GetSkaterPawnMovementComponent`)))
    (`self.OnLandedEvent`)
    (`self.CalculateRideSoundPitch`)
    (else
      (set `self.IsSoundPlaying` false :!label _label)
      (if (`KismetSystemLibrary.IsValid` _ridesoundref)
        (`AudioComponent.Stop` _ridesoundref)))))

(event `self.ReceiveDestroyed`
  (goto _label))

(event `OnLandedEvent`
  (bind _returnvalue (- (`self.K2_GetActorLocation`) (* (`KismetMathLibrary.Vector_Up`) (`CapsuleComponent.GetScaledCapsuleHalfHeight` (`self.CapsuleComponent`)))))
  ;[1 0.5885 0.5885] Play ride sound + Calculate sound location
  (if (not (`self.IsSoundPlaying`))
    (`GameplayStatics.PlaySoundAtLocation` "/Game/SkateTraffic/Audio/Sounds/SW_Skateboard_Land.SW_Skateboard_Land" _returnvalue (struct) 0.5 1.0 0.0 null null null)
    (bind _returnvalue_2 (`GameplayStatics.SpawnSoundAtLocation` "/Game/SkateTraffic/Audio/Sounds/SC_Skateboard_Ride.SC_Skateboard_Ride" _returnvalue (struct) 0.7 (`self.RideSoundPitch`) 0.0 null null))
    (set `self.RideSoundRef` _returnvalue_2)
    (set `self.IsSoundPlaying` true)))

(fn `CalculateRideSoundPitch`
  (bind _returnvalue (- (/ (`KismetMathLibrary.VSize` (`MovementComponent.Velocity` (`self.GetMovementComponent`))) (`STBasePawnMovementComponent.MaxVelocity` (`self.GetSkaterPawnMovementComponent`))) 0.2))
  ;[0.7447 1 0.5677] Calculate ride sound PITCH
  (if (< _returnvalue 0.0)
    (set `self.RideSoundPitch` 1.0)
    (else
      (set `self.RideSoundPitch` (* (+ _returnvalue 1.0) 1.0)))))

(fn `Set Player Camera BlurAndFOV`
  (bind _returnvalue (`self.GetSkaterPawnMovementComponent`))
  (bind _changefovminvelocity (`self.ChangeFOVMinVelocity`))
  (bind _returnvalue_2 (- (`KismetMathLibrary.VSize` (`MovementComponent.Velocity` _returnvalue)) _changefovminvelocity))
  (bind _returnvalue_3 (/ _returnvalue_2 (- (`STBasePawnMovementComponent.MaxVelocity` _returnvalue) _changefovminvelocity)))
  (`CameraComponent.SetFieldOfView` (`self.CameraComponent`) (`self.CurrentFOV`))
  (set `CameraComponent.PostProcessSettings` (make `PostProcessSettings` :`MotionBlurAmount` (`self.CurrentBlur`)) (`self.CameraComponent`))
  (if (< _returnvalue_2 0.0)
    (set `self.CurrentFOV` (`self.DefaultFOV`))
    (set `self.CurrentBlur` (`self.DefaultBlur`))
    (else
      (set `self.CurrentFOV` (`|EaseFunction` "EaseIn" _returnvalue_3 (`self.DefaultFOV`) (`self.MaxFOV`)))
      (set `self.CurrentBlur` (`|EaseFunction` "EaseIn" _returnvalue_3 (`self.DefaultBlur`) (`self.MaxBlur`))))))

(fn `SetMotionBlur`
  (locals (NewLocalVar_0 :type "PostProcessSettings Structure")))

(fn `UserConstructionScript`)