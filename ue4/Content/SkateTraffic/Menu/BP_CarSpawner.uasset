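; BP_CarSpawner is a traffic spawner in the SkateTraffic menu folder that periodically creates random cars in random lanes.
; A looping timer, with its random interval rolled once at BeginPlay, spawns a class from CarsArray at the spawner's transform plus a lane X offset, skipping blocked spots.
; Each spawned car's movement component receives a minimum target speed and its lane number.
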(event `self.ReceiveBeginPlay`
  (`KismetSystemLibrary.K2_SetTimerDelegate` (delegate `SpawnCar`) (`KismetMathLibrary.RandomFloatInRange` 1.0 2.5) true))

(event `SpawnCar`
  (bind _returnvalue (`self.GetTransform`))
  (bind _carsarray (`self.CarsArray`))
  (bind _lanesxlocations (`self.LanesXLocations`))
  (bind _output_get (set `self.LaneNum` (`KismetMathLibrary.RandomInteger` (`KismetArrayLibrary.Array_Length` _lanesxlocations))))
  (bind _returnvalue_2 (`|SpawnActorFromClass` (`|GetArrayItem` _carsarray (`KismetMathLibrary.RandomInteger` (`KismetArrayLibrary.Array_Length` _carsarray))) (`KismetMathLibrary.MakeTransform` (`KismetMathLibrary.MakeVector` (+ (`|GetArrayItem` _lanesxlocations _output_get) (.x (.location _returnvalue))) (.y (.location _returnvalue)) (.z (.location _returnvalue))) (.rotation _returnvalue) (.scale _returnvalue)) "DontSpawnIfColliding" "OverrideRootScale" null null))
  (`/Engine/EditorBlueprintResources/StandardMacros.IsValid` _returnvalue_2
    (:`Is Valid`
      (bind _returnvalue_3 (`CarPawn.GetCarPawnMovementComponent` _returnvalue_2))
      (`CarPawnMovementComponent.SetCarSpeedValues` _returnvalue_3 (make `CarSpeedValues` 1000.0))
      (`STBasePawnMovementComponent.SetCurrentLaneNum` _returnvalue_3 _output_get))))

(fn `UserConstructionScript`)